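; Score component that keeps a running score, shows it in the gameplay widget and saves a best score.
; AddScore increments the total, while UpdateText separately pushes it as text to the first top-level Widget_Gameplay found, then calls an empty effects hook.
; SaveBestScore writes the passed value to a fresh MySaveGame in a dedicated slot, without comparing it to any previous best.
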(fn `AddScore`
  (params (value :type Integer))
  (set `self.Score` (+ value (`self.Score`))))

(fn `SaveBestScore`
  (params (Score :type Integer))
  (bind _returnvalue (`GameplayStatics.CreateSaveGameObject` "/Game/Blueprints/MySaveGame.MySaveGame_C"))
  (set `/Game/Blueprints/MySaveGame.BestScore` Score _returnvalue)
  (`GameplayStatics.SaveGameToSlot` _returnvalue "SaveSlot_BestScore"))

(fn `UpdateText`
  (`self.UpdateText_NewValue`)
  (`self.UpdateText_Effects`))

(fn `UpdateText_Effects`)

(fn `UpdateText_NewValue`
  (bind _foundwidgets (`WidgetBlueprintLibrary.GetAllWidgetsOfClass` "/Game/Blueprints/Widgets/Widget_Gameplay.Widget_Gameplay_C"))
  (set `/Game/Blueprints/Widgets/Widget_Gameplay.txt` (`KismetTextLibrary.Conv_IntToText` (`self.Score`)) (`|GetArrayItem` _foundwidgets)))