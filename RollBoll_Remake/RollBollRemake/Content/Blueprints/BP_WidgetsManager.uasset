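; BP_WidgetsManager switches the game's UI screens between menu, gameplay and game over, showing the menu on BeginPlay.
; Each screen has a function that creates its widget, adds it to the viewport and sets the mouse cursor, which is hidden only during gameplay.
; Matching remove functions find top-level widgets of that class and detach them, rather than keeping stored references.
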(event `self.ReceiveBeginPlay`
  (`self.SetCurrentWidgetToMenu`))

(fn `RemoveWidget_gameover`
  (bind _foundwidgets (`WidgetBlueprintLibrary.GetAllWidgetsOfClass` (`self.GameOverWidget`)))
  (`Widget.RemoveFromParent` _foundwidgets))

(fn `RemoveWidget_gameplay`
  (bind _foundwidgets (`WidgetBlueprintLibrary.GetAllWidgetsOfClass` (`self.GameplayWidget`)))
  (`Widget.RemoveFromParent` _foundwidgets))

(fn `RemoveWidget_menu`
  (bind _foundwidgets (`WidgetBlueprintLibrary.GetAllWidgetsOfClass` (`self.MenuWidget`)))
  (`Widget.RemoveFromParent` _foundwidgets))

(fn `SetCurrentWidgetToGameOver`
  (bind _returnvalue (`|CreateWidget` (`self.GameOverWidget`)))
  (`UserWidget.AddToViewport` _returnvalue 0)
  (set `PlayerController.bShowMouseCursor` true (`GameplayStatics.GetPlayerController` 0)))

(fn `SetCurrentWidgetToGameplay`
  (bind _returnvalue (`|CreateWidget` (`self.GameplayWidget`)))
  (`UserWidget.AddToViewport` _returnvalue 0)
  (set `PlayerController.bShowMouseCursor` false (`GameplayStatics.GetPlayerController` 0)))

(fn `SetCurrentWidgetToMenu`
  (bind _returnvalue (`|CreateWidget` (`self.MenuWidget`)))
  (`UserWidget.AddToViewport` _returnvalue 0)
  (set `PlayerController.bShowMouseCursor` true (`GameplayStatics.GetPlayerController` 0)))

(fn `UserConstructionScript`)