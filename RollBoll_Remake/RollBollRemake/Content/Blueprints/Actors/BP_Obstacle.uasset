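; BP_Obstacle is a self-chaining track segment for an endless-runner style game, with three blocking meshes and randomized beach decorations.
; Construction randomly removes one mesh to leave a gap and optionally drops the detection zone; BeginPlay randomly hides decorations per category.
; When BP_Player enters the zone, it spawns the next obstacle along X, adds score, updates player speed, then self-destructs after a delay.
; Touching a remaining mesh triggers game over.
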(event `self.ReceiveBeginPlay`
  (`self.HandleDecorations` (`self.Chairs`) (`self.int_ChanceOfSpawn_Chairs`))
  (`self.HandleDecorations` (`self.Parasols`) (`self.int_ChanceOfSpawn_Parasols`))
  (`self.HandleDecorations` (`self.Trees`) (`self.int_ChanceOfSpawn_Trees`))
  (`self.HandleDecorations` (`self.Rocks`) (`self.int_ChanceOfSpawn_Rocks`))
  (`self.HandleDecorations` (`self.Sand`) (`self.int_ChanceOfSpawn_Sand`))
  (`self.HandleDecorations` (`self.Docks`) (`self.int_ChanceOfSpawn_Docks`)))

(event `self.DetectionZone.OnComponentBeginOverlap`
  (params (OverlappedComponent :type "PrimitiveComponent Object Reference") (OtherActor :type "Actor Object Reference") (OtherComp :type "PrimitiveComponent Object Reference") (OtherBodyIndex :type Integer) (bFromSweep :type Boolean) (SweepResult :type "HitResult Structure (by ref)"))
  (bind _asbp_player (cast `/Game/Blueprints/Pawns/BP_Player` OtherActor))
  (`self.SpawnNewObstacle`)
  (bind _bp_scorecomponent (`/Game/Blueprints/Pawns/BP_Player.BP_ScoreComponent` _asbp_player))
  (`/Game/Blueprints/BP_ScoreComponent.AddScore` _bp_scorecomponent 1)
  (`/Game/Blueprints/BP_ScoreComponent.UpdateText` _bp_scorecomponent)
  (`/Game/Blueprints/Pawns/BP_Player.HandleSpeed` _asbp_player)
  (`ActorComponent.K2_DestroyComponent` (`self.DetectionZone`))
  (`KismetSystemLibrary.Delay` 1.5)
  (`self.K2_DestroyActor`))

(event `self.StaticMesh.OnComponentBeginOverlap`
  (params (OverlappedComponent :type "PrimitiveComponent Object Reference") (OtherActor :type "Actor Object Reference") (OtherComp :type "PrimitiveComponent Object Reference") (OtherBodyIndex :type Integer) (bFromSweep :type Boolean) (SweepResult :type "HitResult Structure (by ref)"))
  (bind _asbp_player (cast `/Game/Blueprints/Pawns/BP_Player` OtherActor))
  (`/Game/Blueprints/Pawns/BP_Player.HandleGameOver` _asbp_player))

(event `self.StaticMesh1.OnComponentBeginOverlap`
  (params (OverlappedComponent :type "PrimitiveComponent Object Reference") (OtherActor :type "Actor Object Reference") (OtherComp :type "PrimitiveComponent Object Reference") (OtherBodyIndex :type Integer) (bFromSweep :type Boolean) (SweepResult :type "HitResult Structure (by ref)"))
  (bind _asbp_player (cast `/Game/Blueprints/Pawns/BP_Player` OtherActor))
  (`/Game/Blueprints/Pawns/BP_Player.HandleGameOver` _asbp_player))

(event `self.StaticMesh2.OnComponentBeginOverlap`
  (params (OverlappedComponent :type "PrimitiveComponent Object Reference") (OtherActor :type "Actor Object Reference") (OtherComp :type "PrimitiveComponent Object Reference") (OtherBodyIndex :type Integer) (bFromSweep :type Boolean) (SweepResult :type "HitResult Structure (by ref)"))
  (bind _asbp_player (cast `/Game/Blueprints/Pawns/BP_Player` OtherActor))
  (`/Game/Blueprints/Pawns/BP_Player.HandleGameOver` _asbp_player))

(fn `HandleDecorations`
  (params (DecorationParent :type "SceneComponent Object Reference") (ChanceOfSpawn :type Integer))
  (for _array_element (`SceneComponent.GetChildrenComponents` DecorationParent true)
    (if (>= (`KismetMathLibrary.RandomIntegerInRange` 0 10) ChanceOfSpawn)
      (`SceneComponent.SetVisibility` _array_element false false))))

(fn `SpawnNewObstacle`
  (bind (_returnvalue_x _returnvalue_y _returnvalue_z) (`KismetMathLibrary.BreakVector` (`self.K2_GetActorLocation`)))
  (`|SpawnActorFromClass` "BP_Obstacle_C" (`KismetMathLibrary.MakeTransform` (`KismetMathLibrary.MakeVector` (+ _returnvalue_x (`self.fDistanceToNewObstacleSpawn`)) _returnvalue_y _returnvalue_z)) "Undefined" "OverrideRootScale" null null))

(fn `UserConstructionScript`
  (switch `int` (`KismetMathLibrary.RandomInteger` 3)
    (:`0`
      (`ActorComponent.K2_DestroyComponent` (`self.StaticMesh`)))
    (:`1`
      (`ActorComponent.K2_DestroyComponent` (`self.StaticMesh1`)))
    (:`2`
      (`ActorComponent.K2_DestroyComponent` (`self.StaticMesh2`))))
  (if (`self.bDontSpawnBox`)
    (`ActorComponent.K2_DestroyComponent` (`self.DetectionZone`))))